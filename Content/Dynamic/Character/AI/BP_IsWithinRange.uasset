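; Behavior Tree decorator that checks whether the AI's controlled pawn is within range of a target actor.
; It reads the actor from the Target blackboard key and passes when the 3D distance between the two actor locations is at most AcceptableRadius.
; The condition returns a result only for a valid target, with no explicit return otherwise.
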(fn `PerformConditionCheckAI`
  (params (OwnerController :type "AIController Object Reference") (ControlledPawn :type "Pawn Object Reference"))
  (returns (ReturnValue :type Boolean))
  (bind _returnvalue (`BTFunctionLibrary.GetBlackboardValueAsActor` (`self.Target`)))
  (`/Engine/EditorBlueprintResources/StandardMacros.IsValid` _returnvalue
    (:`Is Valid`
      (return (<= (`KismetMathLibrary.Abs` (`KismetMathLibrary.VSize` (- (`Actor.K2_GetActorLocation` ControlledPawn) (`Actor.K2_GetActorLocation` _returnvalue)))) (`self.Acceptable Radius`))))))