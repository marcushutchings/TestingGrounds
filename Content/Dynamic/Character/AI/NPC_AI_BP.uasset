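; AI controller for guard robot NPCs that patrols and reacts to perceived targets.
; On begin play it loads the PatrolData blackboard and runs the GuardBehaviour behavior tree.
; Perception updates ignore actors tagged GuardBots, then set or clear the FocusEnemy key based on whether the stimulus is sensed.
; The same sensed state drives the controlled RobotCharacter's FocusOnTarget and FireAtTarget flags.
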(event `self.ReceiveBeginPlay`
  (`self.UseBlackboard` "/Game/Dynamic/Character/AI/PatrolData.PatrolData")
  (`self.RunBehaviorTree` "/Game/Dynamic/Character/AI/GuardBehaviour.GuardBehaviour"))

(event `self.AIPerception.OnTargetPerceptionUpdated`
  (params (Actor :type "Actor Object Reference") (Stimulus :type "AIStimulus Structure"))
  (bind (_age _expirationage _strength _stimuluslocation _receiverlocation _tag _bsuccessfullysensed) (break `AIStimulus` Stimulus))
  (bind _focus_enemy (`self.Focus Enemy`))
  (bind _blackboard (`self.Blackboard`))
  (if (not (`self.ActorHasTag` Actor "GuardBots"))
    (if _bsuccessfullysensed
      (`BlackboardComponent.SetValueAsObject` _blackboard _focus_enemy Actor)
      (else
        (`BlackboardComponent.ClearValue` _blackboard _focus_enemy)))
    (bind _asrobot_character (cast `/Game/Dynamic/Character/Behaviour/RobotCharacter` (`self.K2_GetPawn`)))
    (bind _output_get (set `/Game/Dynamic/Character/Behaviour/RobotCharacter.FocusOnTarget` _bsuccessfullysensed _asrobot_character))
    (set `/Game/Dynamic/Character/Behaviour/RobotCharacter.FireAtTarget` _output_get _asrobot_character)))

(fn `UserConstructionScript`)