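; BP_NPC_AI is an AI controller for guard NPCs that tracks enemies through AI perception.
; On BeginPlay it loads the BB_PatrolData blackboard and runs the BT_GuardBehaviour behavior tree.
; Perception updates set the sensed actor as the FocusEnemy blackboard key, or clear the key when sensing fails.
; Actors tagged GuardBots are ignored, so fellow guards never affect the focus target.
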(event `self.ReceiveBeginPlay`
  (`self.UseBlackboard` "/Game/Dynamic/Character/AI/BB_PatrolData.BB_PatrolData")
  (`self.RunBehaviorTree` "/Game/Dynamic/Character/AI/BT_GuardBehaviour.BT_GuardBehaviour"))

(event `self.AIPerception.OnTargetPerceptionUpdated`
  (params (Actor :type "Actor Object Reference") (Stimulus :type "AIStimulus Structure"))
  (`self.Update Blackboard Enemy Key` Actor Stimulus Actor))

(fn `Update Blackboard Enemy Key`
  (params (ObjectValue :type "Object Object Reference") (AIStimulus :type "AIStimulus Structure (by ref)") (self2 :type "Actor Object Reference"))
  (bind _focus_enemy (`self.Focus Enemy`))
  (bind _blackboard (`self.Blackboard`))
  (if (`self.ActorHasTag` self2 "GuardBots")
    _
    (elif (`.bSuccessfullySensed` (break `AIStimulus` AIStimulus))
      (`BlackboardComponent.SetValueAsObject` _blackboard _focus_enemy ObjectValue)
      (else
        (`BlackboardComponent.ClearValue` _blackboard _focus_enemy)))))

(fn `UserConstructionScript`)