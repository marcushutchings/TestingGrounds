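; NPC AI controller Blueprint that runs guard behaviour and tracks a perceived enemy.
; On BeginPlay it initialises the PatrolData blackboard and runs the GuardBehaviour behavior tree.
; AI Perception updates write any sensed actor without the GuardBots tag to the FocusEnemy key.
; A lost stimulus from such an actor clears that key, without checking whether it is the current focus.
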(event `self.ReceiveBeginPlay`
  (`self.UseBlackboard` "/Game/Dynamic/NPC/AI/PatrolData.PatrolData")
  (`self.RunBehaviorTree` "/Game/Dynamic/NPC/AI/GuardBehaviour.GuardBehaviour"))

(event `self.AIPerception.OnTargetPerceptionUpdated`
  (params (Actor :type "Actor Object Reference") (Stimulus :type "AIStimulus Structure"))
  (bind _focus_enemy (`self.Focus Enemy`))
  (bind _blackboard (`self.Blackboard`))
  (if (`self.ActorHasTag` Actor "GuardBots")
    _
    (elif (`.bSuccessfullySensed` (break `AIStimulus` Stimulus))
      (`BlackboardComponent.SetValueAsObject` _blackboard _focus_enemy Actor)
      (else
        (`BlackboardComponent.ClearValue` _blackboard _focus_enemy)))))

(fn `UserConstructionScript`)