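; Terrain tile for an infinite-terrain mode that scatters randomized containers, rocks, canisters and boxes on BeginPlay and starts with its barrier locked.
; The player entering LockingVolume opens the barrier and turns it green; leaving locks it red again and asks InfiniteTerrainGameMode to spawn another tile.
; The player overlapping DestoryVolume destroys the tile.
; GetConnector exposes the ConnectorArrow's world transform.
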(event `self.LockingVolume.OnComponentBeginOverlap`
  (params (OverlappedComponent :type "PrimitiveComponent Object Reference") (OtherActor :type "Actor Object Reference") (OtherComp :type "PrimitiveComponent Object Reference") (OtherBodyIndex :type Integer) (bFromSweep :type Boolean) (SweepResult :type "HitResult Structure (by ref)"))
  (`self.Is Player Actor` OtherActor)
  (`self.UnlockTile`))

(event `self.LockingVolume.OnComponentEndOverlap`
  (params (OverlappedComponent :type "PrimitiveComponent Object Reference") (OtherActor :type "Actor Object Reference") (OtherComp :type "PrimitiveComponent Object Reference") (OtherBodyIndex :type Integer))
  (`self.Is Player Actor` OtherActor)
  (`self.LockTile`)
  (bind _asinfinite_terrain_game_mode (cast `/Game/Dynamic/InfiniteTerrainGameMode` (`GameplayStatics.GetGameMode`)))
  (`/Game/Dynamic/InfiniteTerrainGameMode.SpawnTile` _asinfinite_terrain_game_mode))

(event `self.ReceiveBeginPlay`
  (`self.LockTile`)
  (`self.PlaceTerrain` "/Game/Dynamic/Terrain/Props/BP_Container.BP_Container_C" 1 3 1.0 1.0 400.0)
  (`self.PlaceTerrain` "/Game/Dynamic/Terrain/Props/BP_Rock1.BP_Rock1_C" 0 4 0.6 3.0 150.0)
  (`self.PlaceTerrain` "/Game/Dynamic/Terrain/Props/BP_Rock2.BP_Rock2_C" 0 4 0.6 3.0 250.0)
  (`self.PlaceTerrain` "/Game/Dynamic/Terrain/Props/BP_Rock3.BP_Rock3_C" 0 4 0.6 3.0 250.0)
  (`self.PlaceTerrain` "/Game/Dynamic/Terrain/Props/BP_Canister.BP_Canister_C" 1 7 1.0 1.0 50.0)
  (`self.PlaceTerrain` "/Game/Dynamic/Terrain/Props/BP_Box.BP_Box_C" 2 4 1.0 1.0 100.0))

(event `self.DestoryVolume.OnComponentBeginOverlap`
  (params (OverlappedComponent :type "PrimitiveComponent Object Reference") (OtherActor :type "Actor Object Reference") (OtherComp :type "PrimitiveComponent Object Reference") (OtherBodyIndex :type Integer) (bFromSweep :type Boolean) (SweepResult :type "HitResult Structure (by ref)"))
  (`self.Is Player Actor` OtherActor)
  (`self.K2_DestroyActor`))

(fn `GetConnector`
  (returns (`Attach Transform` :type "Transform Structure"))
  (return (`SceneComponent.K2_GetComponentToWorld` (`self.ConnectorArrow`))))

(fn `LockTile`
  (bind _barrier (`self.Barrier`))
  (`PrimitiveComponent.SetCollisionEnabled` _barrier "QueryAndPhysics")
  (`PrimitiveComponent.SetMaterial` _barrier 0 "/Game/Dynamic/Terrain/MI_Barrier_Red.MI_Barrier_Red"))

(fn `UnlockTile`
  (bind _barrier (`self.Barrier`))
  (`PrimitiveComponent.SetCollisionEnabled` _barrier "NoCollision")
  (`PrimitiveComponent.SetMaterial` _barrier 0 "/Game/Dynamic/Terrain/MI_Barrier_Green.MI_Barrier_Green"))

(fn `UserConstructionScript`)