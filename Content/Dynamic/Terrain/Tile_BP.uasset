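; Terrain tile Blueprint with a barrier that opens and closes based on the player's presence in a locking volume.
; When the player character enters LockingVolume the Barrier's collision is disabled, and when the player leaves it is restored to query and physics.
; GetConnector exposes the ConnectorArrow's world transform as the tile's connection point.
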(event `self.LockingVolume.OnComponentBeginOverlap`
  (params (OverlappedComponent :type "PrimitiveComponent Object Reference") (OtherActor :type "Actor Object Reference") (OtherComp :type "PrimitiveComponent Object Reference") (OtherBodyIndex :type Integer) (bFromSweep :type Boolean) (SweepResult :type "HitResult Structure (by ref)"))
  (`self.Is Player Actor` OtherActor)
  (`self.UnlockTile`))

(event `self.LockingVolume.OnComponentEndOverlap`
  (params (OverlappedComponent :type "PrimitiveComponent Object Reference") (OtherActor :type "Actor Object Reference") (OtherComp :type "PrimitiveComponent Object Reference") (OtherBodyIndex :type Integer))
  (`self.Is Player Actor` OtherActor)
  (`self.LockTile`))

(fn `GetConnector`
  (returns (`Attach Transform` :type "Transform Structure"))
  (return (`SceneComponent.K2_GetComponentToWorld` (`self.ConnectorArrow`))))

(fn `LockTile`
  (`PrimitiveComponent.SetCollisionEnabled` (`self.Barrier`) "QueryAndPhysics"))

(fn `UnlockTile`
  (`PrimitiveComponent.SetCollisionEnabled` (`self.Barrier`) "NoCollision"))

(fn `UserConstructionScript`)